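; Gameplay ability that makes an AI robot fire one projectile at the player robot.
; On activation it yaws the weapon mesh toward the player using a flattened 2D direction, while the shot keeps the full 3D direction.
; The projectile spawns offset from the robot's start point, with configurable speed and the robot as instigator.
; The ability ends immediately after the spawn attempt or a failed avatar cast.
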(event Ability|EventActivateAbility
  (bind _asairobot (Utilities|Casting|CastToAIRobot (.AvatarActor (Utilities|Struct|BreakGameplayAbilityActorInfo (Ability|GetActorInfo))))
    (:then
      (bind _output_get (Variables|Default|SetProjectileVector (- (Transformation|GetActorLocation (Variables|/Script/Project_AP.AIRobot|GetPlayerRobot _asairobot)) (Transformation|GetActorLocation _asairobot))))
      (bind _returnvalue (Class|AIRobot|GetWeaponMeshComponent _asairobot))
      (Transformation|SetWorldRotation _returnvalue (Math|Conversions|RotationFromXVector (Class|KismetMathLibrary|VectorNormal2D _output_get 0.0001)) false false)
      (bind _returnvalue_2 (Game|SpawnActorfromClass (Variables|Default|GetProjectile) (Math|Transform|MakeTransform (+ (Transformation|GetWorldLocation (Class|AIRobot|GetProjectileStartPoint _asairobot)) (* (Math|Vector|Normalize _output_get) (Variables|Default|GetLaunchOffset))) (Math|Conversions|RotationFromXVector (Math|Vector|Normalize _output_get)) "1.000000,1.000000,1.000000") "AdjustIfPossibleButDontSpawnIfColliding" 0 (Variables|Default|GetProjectileSpeed) 0.0 0.0 _asairobot))
      (Ability|EndAbility))
    (:CastFailed
      (Ability|EndAbility))))

(event Ability|EventOnEndAbility
  (params (bWasCancelled :type Boolean)))
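; Gameplay ability that fires a projectile from the player robot and ends immediately.
; On activation it commits, then reads the input vector from the robot's WeaponComponent to aim.
; The projectile spawns offset from the robot's start point along that direction, tilted upward by adding LaunchAngle/90 to Z.
; Input magnitude scales the initial speed, and the robot is set as instigator.
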(event Ability|EventActivateAbility
  (bind _returnvalue (Ability|GetActorInfo))
  (bind _avataractor (Utilities|Struct|BreakGameplayAbilityActorInfo _returnvalue))
  (bind _asplayer_robot (Utilities|Casting|CastToPlayerRobot _avataractor))
  (Variables|Default|SetAs%20Player%20Robot _asplayer_robot)
  (Ability|CommitAbility)
  (bind _output_get (Variables|Default|SetPlayerInput (Class|WeaponComponent|GetPlayerInputVector (Variables|/Script/Project_AP.PlayerRobot|GetWeaponComponent _asplayer_robot))))
  (Variables|Default|SetProjectileVector (+ (Math|Vector|Normalize _output_get) (Math|Vector|MakeVector 0.0 0.0 (/ (Variables|Default|GetLaunchAngle) 9e+01))))
  (Game|SpawnActorfromClass (Variables|Default|GetProjectile) (Math|Transform|MakeTransform (+ (* (Math|Vector|Normalize _output_get) (Variables|Default|GetLaunchOffset)) (Transformation|GetWorldLocation (Class|PlayerRobot|GetProjectileStartPoint (Variables|Default|GetAs%20Player%20Robot)))) (Math|Conversions|RotationFromXVector (+ (Math|Vector|Normalize _output_get) (Math|Vector|MakeVector 0.0 0.0 (/ (Variables|Default|GetLaunchAngle) 9e+01)))) "1.000000,1.000000,1.000000") "AdjustIfPossibleButDontSpawnIfColliding" 0 (* (Variables|Default|GetProjectileSpeed) (Math|Vector|VectorLength (Variables|Default|GetPlayerInput))) 0.0 (Variables|Default|GetAs%20Player%20Robot))
  (Ability|EndAbility))

(event Ability|EventOnEndAbility
  (params (bWasCancelled :type Boolean)))
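; Gameplay ability for the robot's ultimate, which fires a rapid burst of five projectiles in one direction.
; On activation it commits, then caches the aim vector from the player robot's WeaponComponent.
; A RepeatAction task spawns each gravity-free projectile at an offset from the robot's projectile start point along that aim.
; When the burst finishes, it ends the ability and clears the weapon's attacking flag.
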(event Ability|EventActivateAbility
  (bind _returnvalue (Ability|GetActorInfo))
  (bind _avataractor (Utilities|Struct|BreakGameplayAbilityActorInfo _returnvalue))
  (bind _asplayer_robot (Utilities|Casting|CastToPlayerRobot _avataractor))
  (Ability|CommitAbility)
  (Variables|Default|SetPlayer%20Robot _asplayer_robot)
  (bind _output_get (Variables|Default|SetPlayerInput (Class|WeaponComponent|GetPlayerInputVector (Variables|/Script/Project_AP.PlayerRobot|GetWeaponComponent _asplayer_robot))))
  (Variables|Default|SetProjectileVector _output_get)
  (|RepeatAction 0.1 5
    (:OnPerformAction
      (bind _returnvalue_2 (Game|SpawnActorfromClass (Variables|Default|GetProjectile) (Math|Transform|MakeTransform (+ (* (Math|Vector|Normalize _output_get) (Variables|Default|GetLaunchOffset)) (Transformation|GetWorldLocation (Class|PlayerRobot|GetProjectileStartPoint _asplayer_robot))) (Math|Conversions|RotationFromXVector (Math|Vector|Normalize _output_get)) "1.000000,1.000000,1.000000") "AdjustIfPossibleButDontSpawnIfColliding" 0 (* (Variables|Default|GetProjectileSpeed) (Math|Vector|VectorLength (Math|Vector|Normalize _output_get))) 0.0 _asplayer_robot))
      (Variables|/Script/Engine.ProjectileMovementComponent|SetProjectileGravityScale (Class|Projectile|GetProjectileMovement _returnvalue_2) 0.0))
    (:OnFinished
      (Ability|EndAbility)
      (Class|WeaponComponent|SetIsAttacking (Variables|/Script/Project_AP.PlayerRobot|GetWeaponComponent (Variables|Default|GetPlayer%20Robot)) false))))

(event Ability|EventOnEndAbility
  (params (bWasCancelled :type Boolean)))
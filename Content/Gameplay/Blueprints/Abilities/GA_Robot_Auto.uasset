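; Gameplay ability that fires a single projectile from the player robot along the weapon component's input vector.
; On activation it commits, then spawns the projectile offset from the robot's start point, with upward tilt added from LaunchAngle.
; Initial speed scales with input magnitude, and spawning is skipped if collision adjustment fails.
; The robot is set as instigator, and the ability ends immediately after spawning.
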(event Ability|EventActivateAbility
  (bind _returnvalue (Ability|GetActorInfo))
  (bind _avataractor (Utilities|Struct|BreakGameplayAbilityActorInfo _returnvalue))
  (bind _asplayer_robot (Utilities|Casting|CastToPlayerRobot _avataractor))
  (Ability|CommitAbility)
  (bind _output_get (Variables|Default|SetPlayerInput (Class|WeaponComponent|GetPlayerInputVector (Variables|/Script/Project_AP.PlayerRobot|GetWeaponComponent _asplayer_robot))))
  (Variables|Default|SetProjectileVector (+ (Math|Vector|Normalize _output_get) (Math|Vector|MakeVector 0.0 0.0 (/ (Variables|Default|GetLaunchAngle) 9e+01))))
  (Game|SpawnActorfromClass (Variables|Default|GetProjectile) (Math|Transform|MakeTransform (+ (* (Math|Vector|Normalize _output_get) (Variables|Default|GetLaunchOffset)) (Transformation|GetWorldLocation (Class|PlayerRobot|GetProjectileStartPoint _asplayer_robot))) (Math|Conversions|RotationFromXVector (+ (Math|Vector|Normalize _output_get) (Math|Vector|MakeVector 0.0 0.0 (/ (Variables|Default|GetLaunchAngle) 9e+01)))) "1.000000,1.000000,1.000000") "AdjustIfPossibleButDontSpawnIfColliding" 0 (* (Variables|Default|GetProjectileSpeed) (Math|Vector|VectorLength (Variables|Default|GetPlayerInput))) _asplayer_robot)
  (Ability|EndAbility))

(event Ability|EventOnEndAbility
  (params (bWasCancelled :type Boolean)))